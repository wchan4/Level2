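; BP_AdvancedTurret is an enemy turret that turns toward the player on sight and fires BP_AdvancedBullet.
; Each PawnSensing sighting aims the actor from its barrel at the player camera and runs a two-second Delay before spawning a bullet, which throttles fire.
; TakeBulletDamage passes damage to the health-bar widget, which holds health.
; At zero health it awards coins and destroys itself, with death or heavy-hit sounds played at the player's location.
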(event `self.ReceiveBeginPlay`
  (bind _asw_enemy_health (cast `/Game/Enemies/InterfaceAndSound/W_EnemyHealth` (`WidgetComponent.GetUserWidgetObject` (`self.HealthBar`))))
  (set `self.HealthWidget` _asw_enemy_health)
  (bind _returnvalue (`GameplayStatics.GetActorOfClass` "/Game/FirstPersonBP/Blueprints/FirstPersonCharacter.FirstPersonCharacter_C"))
  (set `self.Player` _returnvalue))

(event `self.ReceiveActorBeginOverlap`
  (params (OtherActor :type "Actor Object Reference")))

(event `self.PawnSensing.OnSeePawn`
  (params (Pawn :type "Pawn Object Reference"))
  (bind _asfirst_person_character (cast `/Game/FirstPersonBP/Blueprints/FirstPersonCharacter` Pawn))
  (`|ExecutionSequence`
    (:`then_0`
      (`self.K2_SetActorRotation` (`KismetMathLibrary.FindLookAtRotation` (`SceneComponent.K2_GetComponentLocation` (`self.Barrel`)) (`SceneComponent.K2_GetComponentLocation` (`/Game/FirstPersonBP/Blueprints/FirstPersonCharacter.FirstPersonCamera` _asfirst_person_character)))))
    (:`then_1`
      (`KismetSystemLibrary.Delay` 2.0)
      (`|SpawnActorFromClass` "/Game/Enemies/AdvancedEnemies/BP_AdvancedBullet.BP_AdvancedBullet_C" (`SceneComponent.K2_GetComponentToWorld` (`self.BulletSpawner`)) "Undefined" "OverrideRootScale" null null))))

(fn `TakeBulletDamage`
  (params (Damage :type "Float (double-precision)" :default 0.0))
  (bind _healthwidget (`self.HealthWidget`))
  (bind _returnvalue (`self.K2_GetActorLocation` (`self.Player`)))
  (`/Game/Enemies/InterfaceAndSound/W_EnemyHealth.BulletDamage` _healthwidget Damage)
  (if (<= (`/Game/Enemies/InterfaceAndSound/W_EnemyHealth.Health` _healthwidget) 0.0)
    (`/Game/FirstPersonBP/Blueprints/FirstPersonCharacter.UpdatePlayerCoins` (`self.Player`) 150)
    (`GameplayStatics.PlaySoundAtLocation` "/Game/Enemies/InterfaceAndSound/DeathSound.DeathSound" _returnvalue (struct) 1.0 1.0 0.0 null null null)
    (`self.K2_DestroyActor`)
    (elif (>= Damage 10.0)
      (`GameplayStatics.PlaySoundAtLocation` "/Game/Enemies/InterfaceAndSound/DamageSound.DamageSound" _returnvalue (struct) 1.0 1.0 0.0 null null null))))

(fn `UserConstructionScript`)