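; BP_SpikeTrap is a trap actor that thrusts spikes out and damages the player pawn.
; Player overlap sets an Activated flag and, after a short delay, moves the spikes by a Displacement offset with sweep; leaving reverses the move after another delay.
; A separate SpikeCollision overlap calls UpdatePlayerHealth on the FirstPersonCharacter once per contact, using a Damageable flag that re-arms when any overlap with it ends.
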(event `self.ReceiveActorBeginOverlap`
  (params (OtherActor :type "Actor Object Reference"))
  (bind _spikes (`self.Spikes`))
  (if (== OtherActor (`GameplayStatics.GetPlayerPawn` 0))
    (if (not (`self.Activated`))
      (set `self.Activated` true)
      (`KismetSystemLibrary.Delay` 1.0)
      (`SceneComponent.K2_SetWorldTransform` _spikes (`KismetMathLibrary.MakeTransform` (+ (`SceneComponent.K2_GetComponentLocation` _spikes) (`self.Displacement`))) true false))))

(event `self.ReceiveTick`
  (params (DeltaSeconds :type "Float (single-precision)")))

(event `self.ReceiveActorEndOverlap`
  (params (OtherActor :type "Actor Object Reference"))
  (bind _spikes (`self.Spikes`))
  (if (== OtherActor (`GameplayStatics.GetPlayerPawn` 0))
    (if (`self.Activated`)
      (`KismetSystemLibrary.Delay` 0.5)
      (`SceneComponent.K2_SetWorldTransform` _spikes (`KismetMathLibrary.MakeTransform` (- (`SceneComponent.K2_GetComponentLocation` _spikes) (`self.Displacement`))) true false)
      (set `self.Activated` false))))

(event `self.SpikeCollision.OnComponentBeginOverlap`
  (params (OverlappedComponent :type "PrimitiveComponent Object Reference") (OtherActor :type "Actor Object Reference") (OtherComp :type "PrimitiveComponent Object Reference") (OtherBodyIndex :type Integer) (bFromSweep :type Boolean) (SweepResult :type "HitResult Structure (by ref)"))
  (if (== OtherActor (`GameplayStatics.GetPlayerPawn` 0))
    (if (`self.Damageable`)
      (set `self.Damageable` false)
      (bind _asfirst_person_character (cast `/Game/FirstPersonBP/Blueprints/FirstPersonCharacter` OtherActor))
      (`/Game/FirstPersonBP/Blueprints/FirstPersonCharacter.UpdatePlayerHealth` _asfirst_person_character (`self.Damage`))
      (`KismetSystemLibrary.PrintString` "SpikeHit"))))

(event `self.SpikeCollision.OnComponentEndOverlap`
  (params (OverlappedComponent :type "PrimitiveComponent Object Reference") (OtherActor :type "Actor Object Reference") (OtherComp :type "PrimitiveComponent Object Reference") (OtherBodyIndex :type Integer))
  (set `self.Damageable` true))

(fn `UserConstructionScript`)